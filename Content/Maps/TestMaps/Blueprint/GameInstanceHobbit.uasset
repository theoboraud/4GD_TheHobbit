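; Game instance for a Hobbit test map that checks whether a path links the player pawn's current map position to the selected one.
; CheckPath compares the current position's outgoing paths with the selected position's incoming paths.
; A match assigns that path to PionPlayer and flags it as reversed.
; It prints a French debug message for success or failure, without starting movement itself.
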(fn CheckPath
  (bind _pionplayer (Variables|Default|GetPionPlayer))
  (LocalVariables|SetPathIsFind false)
  (bind _array_element (Utilities|Array|ForEachLoopwithBreak (Variables|/Game/Maps/TestMaps/Blueprint/BP_Position_Map.BP_Position_Map_C|GetPathsOUT (Variables|Default|GetpositionActuelleCarte)) :!label _label)
    (:LoopBody
      (if (LocalVariables|GetPathIsFind)
        (goto _label Break)
        (else
          (for _array_element_2 (Variables|/Game/Maps/TestMaps/Blueprint/BP_Position_Map.BP_Position_Map_C|GetPathsIN (Variables|Default|GetpositionSelectCarte))
            (if (== _array_element _array_element_2)
              (Variables|/Game/Maps/TestMaps/Blueprint/BP_PiontJoueurMap.BP_PiontJoueurMap_C|SetPath_Ref _pionplayer _array_element_2)
              (Variables|/Game/Maps/TestMaps/Blueprint/BP_PiontJoueurMap.BP_PiontJoueurMap_C|SetIsReverse _pionplayer true)
              (LocalVariables|SetPathIsFind true))))))
    (:Completed
      (if (LocalVariables|GetPathIsFind)
        (Development|PrintString "Demarrer deplacement")
        (else
          (Development|PrintString "pas de chemin"))))))