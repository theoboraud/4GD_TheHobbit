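; Player map token actor that travels along the spline of a referenced path actor, forward or in reverse.
; A timeline alpha maps to distance along the spline, setting the actor's world location and rotation on each update, with play rate derived from a duration variable.
; Tick checks IsReverse and uses a DoOnce per direction to start each run only once.
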(event Custom|Move_On_Path_Reverse
  (bind _piont_mover (Variables|Default|GetPiont_Mover))
  (bind _path_ref (Variables|Default|GetPath_Ref))
  (bind _spline (Variables|/Game/Maps/TestMaps/Blueprint/BP_TrackSpline.BP_TrackSpline_C|GetSpline _path_ref))
  (Components|Timeline|SetPlayRate _piont_mover (/ 1.0 (Variables|Default|GetDuration%20Track%20Speed)))
  (Components|Timeline|SetNewTime _piont_mover 1.0)
  (bind _ratio_progression_path (Timeline|Piont_Mover Reverse)
    (:Update
      (bind _output_get (Variables|Default|SetRatio%20Progression%20Path _ratio_progression_path))
      (Transformation|SetActorLocationAndRotation (Spline|GetLocationatDistanceAlongSpline _spline (Math|Float|Lerp 0.0 (Spline|GetSplineLength _spline) _output_get) "World") (Spline|GetRotationatDistanceAlongSpline _spline (Math|Float|Lerp 0.0 (Spline|GetSplineLength _spline) _output_get) "World")))))

(event Custom|Move_On_Path
  (bind _path_ref (Variables|Default|GetPath_Ref))
  (bind _piont_mover (Variables|Default|GetPiont_Mover))
  (bind _spline (Variables|/Game/Maps/TestMaps/Blueprint/BP_TrackSpline.BP_TrackSpline_C|GetSpline _path_ref))
  (Components|Timeline|SetPlayRate _piont_mover (/ 1.0 (Variables|Default|GetDuration%20Track%20Speed)))
  (Components|Timeline|SetNewTime _piont_mover 0.0)
  (bind _ratio_progression_path (Timeline|Piont_Mover Play)
    (:Update
      (bind _output_get (Variables|Default|SetRatio%20Progression%20Path _ratio_progression_path))
      (Transformation|SetActorLocationAndRotation (Spline|GetLocationatDistanceAlongSpline _spline (Math|Float|Lerp 0.0 (Spline|GetSplineLength _spline) _output_get) "World") (Spline|GetRotationatDistanceAlongSpline _spline (Math|Float|Lerp 0.0 (Spline|GetSplineLength _spline) _output_get) "World")))))

(event EventBeginPlay)

(event Collision|EventActorBeginOverlap
  (params (OtherActor :type Actor%20Object%20Reference)))

(event EventTick
  (params (DeltaSeconds :type Float%20%28single-precision%29))
  (if (Variables|Default|GetIsReverse)
    (Utilities|FlowControl|DoOnce false
      (:Completed
        (CallFunction|MoveonPathReverse)))
    (else
      (Utilities|FlowControl|DoOnce false
        (:Completed
          (CallFunction|MoveonPath))))))

(fn ConstructionScript)