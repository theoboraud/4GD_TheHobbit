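; BP_Position_Map is a map position marker with a colored cube and an overlap box for player pieces.
; Click and UnClick events set the cube material's Color parameter to green and red respectively.
; The first overlap by an actor of exact class BP_PiontJoueurMap is stored in PiontRef through a DoOnce, and the following cast leads to no further logic.
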(event OnComponentBeginOverlap(Box)
  (params (OverlappedComponent :type Primitive%20Component%20Object%20Reference) (OtherActor :type Actor%20Object%20Reference) (OtherComp :type Primitive%20Component%20Object%20Reference) (OtherBodyIndex :type Integer) (bFromSweep :type Boolean) (SweepResult :type Hit%20Result%20Structure%20%28by%20ref%29))
  (if (== (Utilities|GetClass OtherActor) "/Game/Maps/TestMaps/Blueprint/BP_PiontJoueurMap.BP_PiontJoueurMap_C")
    (Utilities|FlowControl|DoOnce false
      (:Completed
        (bind _output_get (Variables|Default|SetPiont%20Ref OtherActor))
        (Utilities|Casting|CastToBP_PiontJoueurMap _output_get)))))

(event Custom|UnClick
  (Rendering|Material|SetVectorParameterValueonMaterials (Variables|Default|GetCube) "Color" "1.000000,0.000000,0.000000"))

(event Custom|Click
  (Rendering|Material|SetVectorParameterValueonMaterials (Variables|Default|GetCube) "Color" "0.000000,1.000000, 0"))

(event EventBeginPlay)

(event Collision|EventActorBeginOverlap
  (params (OtherActor :type Actor%20Object%20Reference)))

(event EventTick
  (params (DeltaSeconds :type Float%20%28single-precision%29)))

(fn ConstructionScript)