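; World map position marker that detects the player's map point arriving and highlights itself under the cursor.
; On HitBox overlap with BP_PiontJoueurMap, a DoOnce sets this as TopDownController's current position, clears movement and selection, flags arrival and sets the map widget's desk button.
; The DoOnce is never reset, so arrival registers only once.
; Cursor hover on Box moves and shows IndicateurOverlap, relying on Visibility blocking.
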(event OnBeginCursorOver(Box)
  (params (TouchedComponent :type Primitive%20Component%20Object%20Reference))
  (bind _indicateuroverlap (Variables|Default|GetIndicateurOverlap))
  ;[1 1 1] Necessite BlockDynamics : Visiblity pour fonctionner
  (Transformation|SetActorLocation _indicateuroverlap (Transformation|GetWorldLocation (Variables|Default|GetDefaultSceneRoot)) false true)
  (Rendering|SetActorHiddenInGame _indicateuroverlap false))

(event OnComponentBeginOverlap(HitBox)
  (params (OverlappedComponent :type Primitive%20Component%20Object%20Reference) (OtherActor :type Actor%20Object%20Reference) (OtherComp :type Primitive%20Component%20Object%20Reference) (OtherBodyIndex :type Integer) (bFromSweep :type Boolean) (SweepResult :type Hit%20Result%20Structure%20%28by%20ref%29))
  (if (== (Utilities|GetClass OtherActor) "/Game/Blueprints/BP_PiontJoueurMap.BP_PiontJoueurMap_C")
    (Utilities|FlowControl|DoOnce false
      (:Completed
        (bind _astop_down_controller (Utilities|Casting|CastToTopDownController (Game|GetPlayerController 0)))
        (Variables|/Game/Blueprints/Gameplay/TopDownController.TopDownController_C|SetCurrentPos _astop_down_controller self)
        (Variables|/Game/Blueprints/Gameplay/TopDownController.TopDownController_C|SetPawnIsMoving _astop_down_controller false)
        (Variables|/Game/Blueprints/Gameplay/TopDownController.TopDownController_C|SetSelectPos _astop_down_controller 0)
        (Variables|/Game/Blueprints/Gameplay/TopDownController.TopDownController_C|SetPawnIsArrived _astop_down_controller true)
        (Default|SetButtonDesk (Variables|/Game/Blueprints/Gameplay/TopDownController.TopDownController_C|GetWidgetWorldMap _astop_down_controller) true)))))

(event OnEndCursorOver(Box)
  (params (TouchedComponent :type Primitive%20Component%20Object%20Reference))
  ;[1 1 1] Necessite BlockDynamics : Visiblity pour fonctionner
  (Rendering|SetActorHiddenInGame (Variables|Default|GetIndicateurOverlap) true))

(event EventBeginPlay)

(event Collision|EventActorBeginOverlap
  (params (OtherActor :type Actor%20Object%20Reference)))

(event EventTick
  (params (DeltaSeconds :type Float%20%28single-precision%29)))

(fn ConstructionScript)