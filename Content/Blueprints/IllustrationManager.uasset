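; IllustrationManager actor shows illustrations on a movable sheet and drives a UI gauge of "engouement" (enthusiasm) with reacting child widgets.
; CallIllustration swaps the texture on a dynamic material and moves the sheet pivot into place; HideIllustration moves it aside.
; ChangeEngouement clamps the value to 0–1, plays an up or down animation and updates the widget.
; The T key triggers an illustration, an enthusiasm drop and the children's reactions.
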(event EventBeginPlay
  (bind _illustration (Variables|Default|GetIllustration))
  (Utilities|FlowControl|Sequence
    (:then_0
      ;[1 1 1] Set up material illustration
      (bind _returnvalue (Rendering|Material|CreateDynamicMaterialInstance _illustration 0 "/Game/Blueprints/ChangeIllustration_mat.ChangeIllustration_mat" "None" :!class /Script/Engine.PrimitiveComponent))
      (bind _output_get (Variables|Default|SetInstance_mat_Illu _returnvalue))
      (Rendering|Material|SetMaterial _illustration 0 _output_get)
      ;[1 1 1] Position depart illustration
      (Transformation|SetRelativeLocation (Variables|Default|GetPivotFeuille) "50.000000,50.000000, 0" false false)
      (Input|EnableInput (Game|GetPlayerController 0)))
    (:then_1
      ;[1 1 1] Creer liste widget_child
      (for _array_element (Components|GetChildrenComponents (Variables|Default|GetWidget) false)
        (bind _aswidget_component (Utilities|Casting|CastToWidgetComponent _array_element))
        (Utilities|Array|Add (Variables|Default|GetWidget_childrens) _aswidget_component)))))

(event Input|KeyboardEvents|T
  (params (Key :type Key%20Structure :default "None"))
  (:Pressed
    (Transformation|SetRelativeLocation (Variables|Default|GetPivotFeuille) "0, 0, 0" false false)
    (CallFunction|CallIllustration 2)
    (Utilities|Casting|CastToUI_engouement (UserInterface|GetWidget (Variables|Default|GetWidget)))
    (CallFunction|ChangeEngouement -0.1)
    (CallFunction|ChildrenReact)))

(fn ConstructionScript)

(fn CallIllustration
  (params (ID_Illustration :type Integer))
  (Rendering|Material|SetTextureParameterValue (Variables|Default|GetInstance_mat_Illu) "Albedo_illu" (Utilities|Array|Get(acopy) (Variables|Default|GetIllustrations) ID_Illustration))
  (Transformation|SetRelativeLocation (Variables|Default|GetPivotFeuille) "0, 0, 0" false false))

(fn HideIllustration
  (Transformation|SetRelativeLocation (Variables|Default|GetPivotFeuille) "50.000000,50.000000, 0" false false))

(fn ChildrenReact
  (for _array_element (Variables|Default|GetWidget_childrens)
    (bind _aswidget_children (Utilities|Casting|CastToWidget_Children (UserInterface|GetWidget _array_element)))
    (Default|PlayReaction _aswidget_children)))

(fn ChangeEngouement
  (params (valueToAdd :type Float%20%28single-precision%29))
  (bind _widget (Variables|Default|GetWidget))
  (bind _returnvalue (UserInterface|GetWidget _widget))
  (bind _output_get (LocalVariables|SetEng_old (Variables|Default|GetEngouement)))
  (if (> _output_get (Math|Float|Clamp(Float) (+ (Variables|Default|GetEngouement) valueToAdd) 0.0))
    (bind _asui_engouement (Utilities|Casting|CastToUI_engouement _returnvalue))
    (Default|PlayEngouementMoins _asui_engouement)
    (elif (< _output_get (Math|Float|Clamp(Float) (+ (Variables|Default|GetEngouement) valueToAdd) 0.0))
      (bind _asui_engouement_2 (Utilities|Casting|CastToUI_engouement _returnvalue))
      (Default|PlayEngouementPlus _asui_engouement_2)))
  (bind _asui_engouement_3 (Utilities|Casting|CastToUI_engouement _returnvalue))
  (bind _output_get_2 (Variables|/Game/Blueprints/UI/UI_engouement.UI_engouement_C|Setengouement _asui_engouement_3 (Math|Float|Clamp(Float) (+ (Variables|Default|GetEngouement) valueToAdd) 0.0)))
  (Variables|Default|SetEngouement _output_get_2))